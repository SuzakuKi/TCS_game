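; BP_Platform is a platform Blueprint with helper logic for following a looping list of waypoints.
; GetTargetPI wraps CurPointIndex around the Points array, and IsReachedTP checks whether the Platform component's relative location is within a small distance of that point.
; The event graph holds no movement logic: BeginPlay and Tick are empty, and two debug prints are unconnected.
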(event `self.ReceiveTick`
  (params (DeltaSeconds :type "Float (single-precision)")))

(event `self.ReceiveBeginPlay`)

(fn `GetTargetPI`
  (returns (ReturnValue :type Integer))
  (return (mod (`self.CurPointIndex`) (`KismetArrayLibrary.Array_Length` (`self.Points`)))))

(fn `IsReachedTP`
  (returns (ReturnValue :type Boolean))
  (return (< (`KismetMathLibrary.Vector_Distance` (`|GetArrayItem` (`self.Points`) (`self.GetTargetPI`)) (`SceneComponent.RelativeLocation` (`self.Platform`))) 10.0)))

(fn `UserConstructionScript`)